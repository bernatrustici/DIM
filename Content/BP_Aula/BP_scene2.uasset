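; Elevator-door actor that opens for the first-person character and moves the player to the level Scene2.
; Overlapping OpenDoor fires once, starting two parallel Delay loops that slide the left and right doors apart in small counted steps.
; The left door runs in its own custom event so both move together, without a Timeline.
; A separate ChangeScene overlap loads the level by name.
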(event OnComponentBeginOverlap(changeScene)
  (params (OverlappedComponent :type Primitive%20Component%20Object%20Reference) (OtherActor :type Actor%20Object%20Reference) (OtherComp :type Primitive%20Component%20Object%20Reference) (OtherBodyIndex :type Integer) (bFromSweep :type Boolean) (SweepResult :type Hit%20Result%20Structure%20%28by%20ref%29))
  (Utilities|Casting|CastToBP_FirstPersonCharacter OtherActor)
  (Game|OpenLevel(byName) "Scene2"))

(event OnComponentBeginOverlap(openDoor)
  (params (OverlappedComponent :type Primitive%20Component%20Object%20Reference) (OtherActor :type Actor%20Object%20Reference) (OtherComp :type Primitive%20Component%20Object%20Reference) (OtherBodyIndex :type Integer) (bFromSweep :type Boolean) (SweepResult :type Hit%20Result%20Structure%20%28by%20ref%29))
  ;[1 1 1] Abre portas de elevador
  (Utilities|Casting|CastToBP_FirstPersonCharacter OtherActor)
  (Utilities|FlowControl|DoOnce false
    (:Completed
      (CallFunction|PortaEsquerda)
      (Transformation|AddLocalOffset (Variables|Default|Getdireita) "2.000000,0.000000,0.000000" false false :!label _label)
      (Utilities|FlowControl|Delay 0.1)
      (bind _result (Math|Integer|IncrementInt (Variables|Default|Getcont))
        (:%20%20
          (if (not (== _result 25))
            (goto _label)))))))

(event Custom|portaEsquerda
  ;[1 1 1] Abre portas de elevador
  (Transformation|AddLocalOffset (Variables|Default|Getesquerda) "-2.000000,0.000000,0.000000" false false :!label _label)
  (Utilities|FlowControl|Delay 0.1)
  (bind _result (Math|Integer|IncrementInt (Variables|Default|Getcont2))
    (:%20%20
      (if (not (== _result 25))
        (goto _label)))))

(event EventBeginPlay)

(event Collision|EventActorBeginOverlap
  (params (OtherActor :type Actor%20Object%20Reference)))

(event EventTick
  (params (DeltaSeconds :type Float%20%28single-precision%29))
  ;[1 1 1] Abre portas de elevador
)

(fn ConstructionScript)